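; Player-controlled tank Blueprint that handles camera aiming and fire input.
; Azimuth and elevation axes rotate the gimbal's yaw and the spring arm's pitch separately, scaled by frame delta time.
; On BeginPlay it passes its turret and barrel components to setter functions, and the Fire action calls Fire, whose logic lives outside these graphs.
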(event `InputAxis|AimAzimuth`
  (params (AxisValue :type "Float (single-precision)"))
  ;[1 1 1] Azimuth
  (`SceneComponent.K2_AddLocalRotation` (`self.Azimuth gimbal`) (`KismetMathLibrary.MakeRotator` 0.0 0.0 (* AxisValue (`GameplayStatics.GetWorldDeltaSeconds`) 6.0)) false false))

(event `InputAxis|AimElevation`
  (params (AxisValue :type "Float (single-precision)"))
  ;[1 1 1] Elevation
  (`SceneComponent.K2_AddLocalRotation` (`self.SpringArm`) (`KismetMathLibrary.MakeRotator` 0.0 (* AxisValue (`GameplayStatics.GetWorldDeltaSeconds`) 6.0)) false false))

(event `self.ReceiveBeginPlay`
  (`self.SetTurrentRefrence` (`self.TankTurrent`))
  (`self.SetBarrelRefrence` (`self.Barrel`)))

(event `InputAction|Fire`
  (params (Key :type "Key Structure"))
  (:`Pressed`
    (`self.Fire`)))

(fn `UserConstructionScript`)